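; Player character Blueprint that forwards player input to inherited-style handler functions for shooting, reloading, quick-switching, horizontal movement, jumping and crouching, with touch sharing the jump path.
; BeginPlay enables controller input, runs parent logic, adds the health HUD to the viewport and clears the dead flag.
; KillSelf zeroes capsule velocity, switches to UI-only input, releases the trigger, disables input and calls parent death logic, ending in a delay with nothing after it.
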(event EventBeginPlay
  ;[1 1 1] Event BeginPlay
  (CallFunction|EnablePlayerControllerInput)
  (|CallParentFunction)
  (bind _returnvalue (UserInterface|CreateWidget "/Game/MyContent/Blueprints/HUD/Widget_Player_Health_HUD.Widget_Player_Health_HUD_C" (Game|GetPlayerController 0)))
  (bind _output_get (Variables|Default|SetHealthBar _returnvalue))
  (UserInterface|Viewport|AddtoViewport _output_get 0)
  (Variables|Default|SetCharIsDead false))

(event EventTick
  (params (DeltaSeconds :type Float%20%28single-precision%29))
  ;[1 1 1] Event Tick
  (|CallParentFunction DeltaSeconds))

(event EventKillSelf
  ;[1 1 1] Kill Self
  (Physics|SetPhysicsLinearVelocity (Variables|Default|GetCapsuleComponent) "0, 0, 0" false "None")
  (Input|SetInputModeUIOnly (Game|GetPlayerController 0) 0 "DoNotLock")
  (CallFunction|InputShootRelease)
  (CallFunction|DisablePlayerControllerInput)
  (|CallParentFunction)
  (Utilities|FlowControl|Delay 3.0))

(event Input|ActionEvents|InputActionShoot
  (params (Key :type Key%20Structure))
  ;[1 1 1] Assigning Inputs
  (:Pressed
    (CallFunction|InputShootPress))
  (:Released
    (CallFunction|InputShootRelease)))

(event Input|ActionEvents|InputActionReload
  (params (Key :type Key%20Structure))
  ;[1 1 1] Assigning Inputs
  (:Released
    (CallFunction|InputReloadRelease)))

(event Input|ActionEvents|InputActionJump
  (params (Key :type Key%20Structure))
  ;[1 1 1] Assigning Inputs
  (:Pressed
    (CallFunction|InputJumpPress))
  (:Released
    (CallFunction|InputJumpRelease)))

(event Input|ActionEvents|InputActionCrouch
  (params (Key :type Key%20Structure))
  ;[1 1 1] Assigning Inputs
  (:Pressed
    (CallFunction|InputCrouchPress))
  (:Released
    (CallFunction|InputCrouchRelease)))

(event Input|AxisEvents|InputAxisMoveRight
  (params (AxisValue :type Float%20%28single-precision%29))
  ;[1 1 1] Assigning Inputs
  (CallFunction|InputMoveRight AxisValue))

(event Input|KeyboardEvents|Q
  (params (Key :type Key%20Structure))
  ;[1 1 1] Assigning Inputs
  (:Pressed
    (CallFunction|InputQuickswitchPress)))

(event Input|TouchEvents|InputTouch
  (params (Location :type Vector) (FingerIndex :type ETouchIndex%20Enum))
  ;[1 1 1] Assigning Inputs
  (:Pressed
    (CallFunction|InputJumpPress))
  (:Released
    (CallFunction|InputJumpRelease)))

(fn ConstructionScript
  (|CallParentFunction))