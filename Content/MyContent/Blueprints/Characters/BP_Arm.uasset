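; BP_Arm is a Paper2D front arm that animates as a separate piece for a character.
; Each tick while alive, it checks that its owner is a BP_Character_Base, then picks the idle, attack, run or draw flipbook from ArmStates.
; Die stops those state updates and plays the dying flipbook, switching to the dead one after a short fixed delay.
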(event Custom|Update%20Animation
  ;[1 1 1] Handle Animation
  (if (Variables|Default|GetAHIsAlive)
    (Utilities|Casting|CastToBP_Character_Base (Components|GetOwner))
    (switch Utilities|FlowControl|Switch|SwitchonArm_States (Variables|Default|GetArmStates)
      (:NewEnumerator0
        (Sprite|SetFlipbook (Variables|Default|GetFrontArmFlipbook) (Variables|Default|GetIdle_FB)))
      (:NewEnumerator5
        (Sprite|SetFlipbook (Variables|Default|GetFrontArmFlipbook) (Variables|Default|GetAttack_FB)))
      (:NewEnumerator7
        (Sprite|SetFlipbook (Variables|Default|GetFrontArmFlipbook) (Variables|Default|GetRun_FB)))
      (:NewEnumerator6
        (Sprite|SetFlipbook (Variables|Default|GetFrontArmFlipbook) (Variables|Default|GetDraw_FB))))))

(event Custom|Die
  ;[1 1 1] Die
  (Variables|Default|SetAHIsAlive false)
  (Sprite|SetFlipbook (Variables|Default|GetFrontArmFlipbook) (Variables|Default|GetDying_FB))
  (Utilities|FlowControl|Delay 0.8)
  (Sprite|SetFlipbook (Variables|Default|GetFrontArmFlipbook) (Variables|Default|GetDead_FB)))

(event EventTick
  (params (DeltaSeconds :type Float%20%28single-precision%29))
  ;[1 1 1] Event Tick
  (CallFunction|UpdateAnimation))

(fn ConstructionScript)