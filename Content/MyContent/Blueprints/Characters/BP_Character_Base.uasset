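; Base 2D Paper2D side-scroller character that builds itself from a body sprite plus socket-attached arm actors and either two guns or a sword.
; Tick yaw-flips the actor by movement direction and sets body and arm flipbook states.
; Input events drive timed automatic fire, reload and crouch, while health loss triggers death and weapon drop.
; Jump press, vault, knockback and quickswitch events are empty, with related logic left disconnected.
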(event OnComponentBeginOverlap(CapsuleComponent)
  (params (OverlappedComponent :type Primitive%20Component%20Object%20Reference) (OtherActor :type Actor%20Object%20Reference) (OtherComp :type Primitive%20Component%20Object%20Reference) (OtherBodyIndex :type Integer) (bFromSweep :type Boolean) (SweepResult :type Hit%20Result%20Structure%20%28by%20ref%29))
  ;[1 1 1] Pickup Gun
  (if (not (Actor|ActorHasTag OtherActor "Gun"))
    (if (Actor|ActorHasTag OtherActor "Bullet")
      _)))

(event OnComponentHit(CapsuleComponent)
  (params (HitComponent :type Primitive%20Component%20Object%20Reference) (OtherActor :type Actor%20Object%20Reference) (OtherComp :type Primitive%20Component%20Object%20Reference) (NormalImpulse :type Vector :default "0, 0, 0") (Hit :type Hit%20Result%20Structure%20%28by%20ref%29))
  ;[1 1 1] Collide with Vaultable Object
)

(event Custom|InitiateGun
  (params (GunType :type Gun_Types%20Enum%20%28by%20ref%29 :default "NewEnumerator0") (IsHeld :type Boolean%20%28by%20ref%29))
  (bind _sprite (Variables|Default|GetSprite))
  ;[1 1 1] Gun Events
  (bind _outputgun (CallFunction|SpawnGun GunType))
  (if IsHeld
    (bind _output_get (Variables|Default|SetHeldGun _outputgun))
    (Transformation|AttachComponentToComponent _output_get _sprite "BobbingPos" "KeepRelative" "KeepRelative" "KeepRelative" true)
    (else
      (bind _output_get_2 (Variables|Default|SetHolsteredGun _outputgun))
      (Transformation|AttachComponentToComponent _output_get_2 _sprite "BobbingPos" "KeepRelative" "KeepRelative" "KeepRelative" true)))
  (CallFunction|LoadGunProperties))

(event Custom|ApplyKnockback
  (params (DamageIn :type Float%20%28single-precision%29) (Direction :type Integer))
  ;[1 1 1] Apply Knockback
)

(event Custom|HideGun
  (params (TargetGun :type BP%20Gun%20Object%20Reference) (IsHidden :type Boolean))
  ;[1 1 1] Gun Events
  (Rendering|SetActorHiddenInGame TargetGun IsHidden))

(event Custom|GunFaceLeft
  ;[1 1 1] Gun Events
  (Default|LeftFacing (Variables|Default|GetHeldGun)))

(event Custom|FireGun
  ;[1 1 1] Gun Events
  (Default|Fire (Variables|Default|GetHeldGun)))

(event Custom|ReloadGun
  ;[1 1 1] Gun Events
  (Default|Reload (Variables|Default|GetHeldGun)))

(event Custom|RemoveHealth
  (params (HealthLost :type Float%20%28single-precision%29))
  ;[1 1 1] Remove Health
  (if (> (Variables|Default|GetHealthCurrent) 0.0)
    (bind _output_get (Variables|Default|SetHealthCurrent (- (Variables|Default|GetHealthCurrent) HealthLost)))
    (Audio|PlaySoundatLocation "/Game/MyContent/Sounds/Voices/voice_male_b_hurt_pain_set_2_06_Cue.voice_male_b_hurt_pain_set_2_06_Cue" (Transformation|GetActorLocation) "0, 0, 0" 1.0 1.0 0.0 0 0 0)
    (if (<= _output_get 0.0)
      (CallFunction|KillSelf))))

(event Custom|SpawnRightHandLeftSide
  ;[1 1 1] Arm Spawning
  (bind _returnvalue (Game|SpawnActorfromClass "/Game/MyContent/Blueprints/Characters/BP_Grunt_RightHandLeftSide.BP_Grunt_RightHandLeftSide_C" (Math|Transform|MakeTransform "0.000000,-4.000000,-55.000000") "Undefined" 0 0))
  (Variables|Default|SetRightHandLeftSide _returnvalue)
  (Transformation|AttachComponentToComponent (Variables|Default|GetRightHandLeftSide) (Variables|Default|GetSprite) "FrontArm" "KeepRelative" "KeepRelative" "KeepRelative" false)
  (Actor|SetOwner (Variables|Default|GetRightHandLeftSide) self))

(event Custom|LoadGunProperties
  (bind _heldgun (Variables|Default|GetHeldGun))
  ;[1 1 1] Load Gun Properties
  (Variables|Default|SetAmmoCount (Variables|/Game/MyContent/Blueprints/Weapons/BP_Gun.BP_Gun_C|GetCurrentAmmo _heldgun))
  (Variables|Default|SetAmmoMax (Variables|/Game/MyContent/Blueprints/Weapons/BP_Gun.BP_Gun_C|GetMaxAmmo _heldgun))
  (Variables|Default|SetAmmoReserve (Variables|/Game/MyContent/Blueprints/Weapons/BP_Gun.BP_Gun_C|GetReserveAmmo _heldgun))
  (Variables|Default|SetIsWeaponAutomatic (Variables|/Game/MyContent/Blueprints/Weapons/BP_Gun.BP_Gun_C|GetIsAutomatic _heldgun)))

(event Custom|InputShootPress
  ;[1 1 1] Shooting
  (if (not (Variables|Default|GetFireCooldown))
    (Variables|Default|SetFireCont true)
    (Variables|Default|SetIsFirstShot true)
    (CallFunction|FireGun)
    (Variables|Default|SetIsFirstShot false)
    (Utilities|FlowControl|Delay (Variables|Default|GetHeldGunFireRate))
    (if (Variables|Default|GetIsWeaponAutomatic)
      (if (Variables|Default|GetFireCont) :!label _label
        (CallFunction|FireGun)
        (Utilities|FlowControl|Delay (Variables|Default|GetHeldGunFireRate))
        (goto _label)))))

(event Custom|UpdateAnimation
  (bind _rightarm_front_ (Variables|Default|GetRightArm%28Front%29))
  ;[1 1 1] Handle Animation
  (if (not (Variables|Default|GetCharIsDead))
    (Variables|/Game/MyContent/Blueprints/Weapons/BP_Sword.BP_Sword_C|SetStates (Variables|Default|GetSword) (Variables|Default|GetStates))
    (if (> (Math|Float|Absolute(Float) (.X (Math|Vector|BreakVector (Variables|/Script/Engine.MovementComponent|GetVelocity (Pawn|GetMovementComponent))))) 0.0)
      (Variables|Default|SetStates "NewEnumerator1")
      (else
        (Variables|Default|SetStates "NewEnumerator0")))
    (Variables|Default|SetPrevState (Variables|Default|GetStates))
    (switch Utilities|FlowControl|Switch|SwitchonCharacter_States (Variables|Default|GetStates)
      (:NewEnumerator0
        (Sprite|SetFlipbook (Variables|Default|GetSprite) (Variables|Default|GetIdleFB))
        (Development|PrintString "Idle")
        (if (not (Variables|Default|GetRightHandBusy))
          (Variables|/Game/MyContent/Blueprints/Characters/BP_Arm.BP_Arm_C|SetArmStates (Variables|Default|GetRightArm%28Front%29) "NewEnumerator0")
          (if (not (Variables|Default|GetLeftHandBusy))
            (Variables|/Game/MyContent/Blueprints/Characters/BP_Arm.BP_Arm_C|SetArmStates (Variables|Default|GetLeftArm%28Back%29) "NewEnumerator0")
            (if (Utilities|Enum|NotEqual(Enum) (Variables|Default|GetStates) (Variables|Default|GetPrevState)) :!label _label
              (CallFunction|PlayFBfromStart)))))
      (:NewEnumerator1
        (Sprite|SetFlipbook (Variables|Default|GetSprite) (Variables|Default|GetRunFB))
        (Development|PrintString "Running")
        (if (not (Variables|Default|GetRightHandBusy))
          (if (Variables|Default|GetSwordDrawn)
            (Variables|/Game/MyContent/Blueprints/Characters/BP_Arm.BP_Arm_C|SetArmStates _rightarm_front_ "NewEnumerator5")
            (else
              (Variables|/Game/MyContent/Blueprints/Characters/BP_Arm.BP_Arm_C|SetArmStates _rightarm_front_ "NewEnumerator7")))
          (if (not (Variables|Default|GetLeftHandBusy))
            (Variables|/Game/MyContent/Blueprints/Characters/BP_Arm.BP_Arm_C|SetArmStates (Variables|Default|GetLeftArm%28Back%29) "NewEnumerator7")
            (goto _label)))))))

(event Custom|Restock%20Ammo
  ;[1 1 1] Restock Ammo
  (Default|RestockAmmo (Variables|Default|GetHolsteredGun))
  (Default|RestockAmmo (Variables|Default|GetHeldGun)))

(event Custom|KillArmHand
  ;[1 1 1] Arm Spawning
  (Default|Die (Variables|Default|GetArmHand)))

(event Custom|InputShootRelease
  ;[1 1 1] Shooting
  (Variables|Default|SetFireCont false)
  (Variables|Default|SetFireCooldown true)
  (Utilities|FlowControl|Delay (Variables|Default|GetHeldGunFireRate))
  (Variables|Default|SetFireCooldown false))

(event Custom|Kill%20Self
  ;[1 1 1] Kill Self
  (Variables|Default|SetCharIsDead true)
  (CallFunction|DropWeapon)
  (Default|EnableGravity (Variables|Default|GetHeldGun))
  (Sprite|SetFlipbook (Variables|Default|GetSprite) (Variables|Default|GetDyingFB))
  (CallFunction|UpdateAnimation)
  (CallFunction|KillArmHand)
  (Utilities|FlowControl|Delay 0.8)
  (Sprite|SetFlipbook (Variables|Default|GetSprite) (Variables|Default|GetDeadFB))
  (CallFunction|UpdateAnimation))

(event Custom|Input%20Quickswitch%20Press
  ;[1 1 1] Quickswitch
)

(event Custom|InputMoveRight
  (params (AxisValue :type Float%20%28single-precision%29))
  ;[1 1 1] Handle Movement
  (if (> AxisValue 0.0)
    (Variables|Default|SetIsMovingRight true)
    (elif (< AxisValue 0.0)
      (Variables|Default|SetIsMovingRight false)))
  (Pawn|Input|AddMovementInput "1.000000, 0, 0" AxisValue false))

(event Custom|InputReloadRelease
  ;[1 1 1] Reloading
  (if (not (Variables|Default|GetIsReloading))
    (if (not (>= (Variables|Default|GetAmmoCount) (Variables|Default|GetAmmoMax)))
      (if (> (Variables|Default|GetAmmoReserve) 0)
        (Variables|Default|SetFireCont false)
        (Utilities|FlowControl|Delay 0.2)
        (Variables|Default|SetIsReloading true)
        (Utilities|FlowControl|Sequence
          (:then_0
            (CallFunction|ReloadGun)))))))

(event Custom|DropWeapon
  ;[1 1 1] Drop Weapon
  (Transformation|DetachFromComponent (Variables|/Script/Engine.Actor|GetRootComponent (Variables|Default|GetHeldGun)) "KeepWorld" "KeepWorld" "KeepWorld" true))

(event Custom|Input%20Jump%20Press
  ;[1 1 1] Handle Jump
)

(event Custom|Vault
  ;[1 1 1] Vault
)

(event Custom|Input%20Jump%20Release
  ;[1 1 1] Handle Jump
  (Character|StopJumping))

(event Custom|UpdateArms
  ;[1 1 1] Arm Spawning
  (Default|UpdateAnimation (Variables|Default|GetRightArm%28Front%29))
  (Default|UpdateAnimation (Variables|Default|GetLeftArm%28Back%29)))

(event Custom|SpawnSword
  ;[1 1 1] Arm Spawning
  (bind _returnvalue (Game|SpawnActorfromClass "/Game/MyContent/Blueprints/Weapons/BP_Sword.BP_Sword_C" (Math|Transform|MakeTransform "0.000000,-4.000000,0.000000") "Undefined" self 0))
  (Variables|Default|SetSword _returnvalue)
  (Transformation|AttachComponentToComponent (Variables|Default|GetSword) (Variables|Default|GetSprite) "Sword" "KeepRelative" "KeepRelative" "KeepRelative" false)
  (Components|MoveComponentTo (Variables|Default|GetDirection) "14.000000,0.000000,25.000000" "0, 0, 0" false false 0.0 false)
  (Transformation|AttachComponentToComponent (Variables|Default|GetDirection) (Variables|Default|GetSprite) "Sword" "KeepRelative" "KeepRelative" "KeepRelative" false))

(event Custom|Input%20Crouch%20Press
  ;[1 1 1] Handle Crouch
  (Character|Crouch)
  (Variables|Default|SetStates "NewEnumerator8")
  (CallFunction|UpdateAnimation)
  (CallFunction|HideGun (Variables|Default|GetHeldGun) true))

(event Custom|Input%20Crouch%20Release
  ;[1 1 1] Handle Crouch
  (Character|UnCrouch)
  (Variables|Default|SetStates "NewEnumerator0")
  (CallFunction|UpdateAnimation)
  (CallFunction|HideGun (Variables|Default|GetHeldGun) false))

(event Custom|DisablePlayerControllerInput
  ;[1 1 1] Enable/Disable Player Controller Input
  (if (Variables|Default|GetIsPlayer)
    (Input|DisableInput (Game|GetPlayerController 0))))

(event Custom|EnablePlayerControllerInput
  ;[1 1 1] Enable/Disable Player Controller Input
  (if (Variables|Default|GetIsPlayer)
    (Input|EnableInput (Game|GetPlayerController 0))))

(event Custom|DrawSword
  ;[1 1 1] Draw Sword
  (Variables|Default|SetRightHandBusy true)
  (Variables|/Game/MyContent/Blueprints/Characters/BP_Arm.BP_Arm_C|SetArmStates (Variables|Default|GetRightArm%28Front%29) "NewEnumerator6")
  (Utilities|FlowControl|Delay 0.375)
  (CallFunction|SpawnRightHandLeftSide)
  (Rendering|SetActorHiddenInGame (Variables|Default|GetSword) true)
  (Variables|Default|SetSwordDrawn true)
  (Utilities|FlowControl|Delay 0.625)
  (Variables|Default|SetRightHandBusy false)
  (Actor|DestroyActor (Variables|Default|GetRightHandLeftSide))
  (CallFunction|PlayFBfromStart)
  (Default|SpawnSword (Variables|Default|GetRightArm%28Front%29)))

(event Custom|SpawnLeftArm
  ;[1 1 1] Arm Spawning
  (bind _returnvalue (Game|SpawnActorfromClass "/Game/MyContent/Blueprints/Characters/BP_Grunt_LeftArm.BP_Grunt_LeftArm_C" (Math|Transform|MakeTransform "0.000000,-6.000000,0.000000") "Undefined" 0 0))
  (Variables|Default|SetLeftArm%28Back%29 _returnvalue)
  (Transformation|AttachComponentToComponent (Variables|Default|GetLeftArm%28Back%29) (Variables|Default|GetSprite) "BackArm" "KeepRelative" "KeepRelative" "KeepRelative" false)
  (Components|MoveComponentTo (Variables|Default|GetDirection) "14.000000,0.000000,25.000000" "0, 0, 0" false false 0.0 false)
  (Actor|SetOwner (Variables|Default|GetLeftArm%28Back%29) self))

(event Custom|PlayFBfromStart
  ;[1 1 1] Play Flipbooks from start
  (Components|Timeline|PlayfromStart (Variables|Default|GetSprite))
  (Components|Timeline|PlayfromStart (Actor|GetComponentbyClass (Variables|Default|GetLeftArm%28Back%29) "/Script/Paper2D.PaperFlipbookComponent"))
  (Components|Timeline|PlayfromStart (Actor|GetComponentbyClass (Variables|Default|GetRightArm%28Front%29) "/Script/Paper2D.PaperFlipbookComponent"))
  (Components|Timeline|PlayfromStart (Actor|GetComponentbyClass (Variables|Default|GetSword) "/Script/Paper2D.PaperFlipbookComponent")))

(event Custom|SpawnRightArm
  ;[1 1 1] Arm Spawning
  (bind _returnvalue (Game|SpawnActorfromClass "/Game/MyContent/Blueprints/Characters/BP_Grunt_RightArm.BP_Grunt_RightArm_C" (Math|Transform|MakeTransform "0.000000,6.000000,0.000000") "Undefined" 0 0))
  (Variables|Default|SetRightArm%28Front%29 _returnvalue)
  (Transformation|AttachComponentToComponent (Variables|Default|GetRightArm%28Front%29) (Variables|Default|GetSprite) "FrontArm" "KeepRelative" "KeepRelative" "KeepRelative" false)
  (Components|MoveComponentTo (Variables|Default|GetDirection) "14.000000,0.000000,25.000000" "0, 0, 0" false false 0.0 false)
  (Actor|SetOwner (Variables|Default|GetRightArm%28Front%29) self))

(event Custom|GunFaceRight
  ;[1 1 1] Gun Events
  (Default|RightFacing (Variables|Default|GetHeldGun)))

(event EventOnLanded
  (params (Hit :type Hit%20Result%20Structure%20%28by%20ref%29))
  ;[1 1 1] Handle Jump
)

(event EventBeginPlay
  ;[1 1 1] Event Begin Play
  (Utilities|FlowControl|Sequence
    (:then_0
      (Class|ActorComponent|SetIsReplicated (Variables|Default|GetSprite) true))
    (:then_1
      (CallFunction|SpawnRightArm)
      (CallFunction|SpawnLeftArm)
      (if (Variables|Default|GetHasGun)
        (CallFunction|InitiateGun (Variables|Default|GetHeldGunType) (Variables|Default|GetIsHeld))
        (bind _output_get (Variables|Default|SetIsHeld false))
        (CallFunction|InitiateGun (Variables|Default|GetHolsteredGunType) _output_get)
        (CallFunction|HideGun (Variables|Default|GetHolsteredGun) true)
        (Variables|Default|SetHeldGunFireRate (Variables|/Game/MyContent/Blueprints/Weapons/BP_Gun.BP_Gun_C|GetMaxFireRate (Variables|Default|GetHeldGun)))
        (else
          (CallFunction|SpawnSword)
          (CallFunction|PlayFBfromStart))))))

(event EventTick
  (params (DeltaSeconds :type Float%20%28single-precision%29))
  ;[1 1 1] Event Tick
  (Variables|Default|SetPrevFacing (Variables|Default|GetFacing))
  (if (not (Variables|Default|GetIsHit))
    (CallFunction|UpdateAnimation)
    (Math|Float|CompareFloat (.X (Math|Vector|BreakVector (Variables|/Script/Engine.MovementComponent|GetVelocity (Pawn|GetMovementComponent)))) 0.0
      (:>
        (Transformation|SetActorRotation (Math|Rotator|MakeRotator 0.0 0.0 0.0) :!label _label)
        (Variables|Default|SetFacing 1))
      (:==
        (if (Variables|Default|GetIsMovingRight)
          (goto _label)
          (else
            (Transformation|SetActorRotation (Math|Rotator|MakeRotator 0.0 0.0 1.8e+02) :!label _label_2)
            (Variables|Default|SetFacing -1))))
      (:<
        (goto _label_2)))))

(event Input|KeyboardEvents|LeftShift
  (params (Key :type Key%20Structure))
  (bind _charactermovement (Variables|Character|GetCharacterMovement))
  ;[1 1 1] Dev-Only Sprint Mechanic
  (:Pressed
    (Variables|/Script/Engine.CharacterMovementComponent|SetMaxWalkSpeed _charactermovement 1e+02))
  (:Released
    (Variables|/Script/Engine.CharacterMovementComponent|SetMaxWalkSpeed _charactermovement 35.0)))

(fn ConstructionScript)

(fn SpawnGun
  (params (Gun%20Type :type Gun_Types%20Enum%20%28by%20ref%29 :default "NewEnumerator0"))
  (switch Utilities|FlowControl|Switch|SwitchonGun_Types Gun%20Type
    (:NewEnumerator0
      (bind _returnvalue (Game|SpawnActorfromClass "/Game/MyContent/Blueprints/Weapons/BP_Ak47.BP_Ak47_C" (Math|Transform|MakeTransform "4.000000,1.000000,24.000000") "Undefined" self 0))
      (return _returnvalue))
    (:NewEnumerator1
      (bind _returnvalue_2 (Game|SpawnActorfromClass "/Game/MyContent/Blueprints/Weapons/BP_Shotgun.BP_Shotgun_C" (Math|Transform|MakeTransform "4.000000,1.000000,24.000000") "Undefined" self 0))
      (return _returnvalue_2))
    (:NewEnumerator2
      (bind _returnvalue_3 (Game|SpawnActorfromClass "/Game/MyContent/Blueprints/Weapons/BP_M4.BP_M4_C" (Math|Transform|MakeTransform "3.000000,1.000000,25.000000") "Undefined" self 0))
      (return _returnvalue_3))
    (:NewEnumerator3
      (bind _returnvalue_4 (Game|SpawnActorfromClass "/Game/MyContent/Blueprints/Weapons/BP_Grenade_Launcher.BP_Grenade_Launcher_C" (Math|Transform|MakeTransform "4.000000,1.000000,24.000000") "Undefined" self 0))
      (return _returnvalue_4))))