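; Enemy character Blueprint that patrols horizontally by driving inherited movement input each tick while alive, reversing direction whenever its capsule hits something.
; On death it releases fire, destroys capsule and sight components, runs the parent kill logic, and shifts the arm and sprite to fixed Y depths.
; Sight overlap events are empty; player-detection shooting, auto-reload and health widget linking exist only as disconnected, never-run logic.
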(event OnComponentHit(CapsuleComponent)
  (params (HitComponent :type Primitive%20Component%20Object%20Reference) (OtherActor :type Actor%20Object%20Reference) (OtherComp :type Primitive%20Component%20Object%20Reference) (NormalImpulse :type Vector :default "0, 0, 0") (Hit :type Hit%20Result%20Structure%20%28by%20ref%29))
  ;[1 1 1] On Component Hit
  (bind _output_get (Variables|Default|SetMoveDirection (* (stale _output_get) -1.0))))

(event OnComponentEndOverlap(Sight)
  (params (OverlappedComponent :type Primitive%20Component%20Object%20Reference) (OtherActor :type Actor%20Object%20Reference) (OtherComp :type Primitive%20Component%20Object%20Reference) (OtherBodyIndex :type Integer))
  ;[1 1 1] Vision
)

(event OnComponentBeginOverlap(Sight)
  (params (OverlappedComponent :type Primitive%20Component%20Object%20Reference) (OtherActor :type Actor%20Object%20Reference) (OtherComp :type Primitive%20Component%20Object%20Reference) (OtherBodyIndex :type Integer) (bFromSweep :type Boolean) (SweepResult :type Hit%20Result%20Structure%20%28by%20ref%29))
  ;[1 1 1] Vision
)

(event EventBeginPlay
  ;[1 1 1] Event BeginPlay
  (|CallParentFunction))

(event EventTick
  (params (DeltaSeconds :type Float%20%28single-precision%29))
  ;[1 1 1] Event Tick
  (|CallParentFunction DeltaSeconds)
  (if (not (Variables|Default|GetCharIsDead))
    (CallFunction|InputMoveRight (Variables|Default|GetMoveDirection))))

(event EventKillSelf
  (bind _armhand (Variables|Default|GetArmHand))
  (bind _sprite (Variables|Default|GetSprite))
  (bind _returnvalue (Transformation|GetActorTransform _armhand))
  (bind _relativelocation (Variables|/Script/Engine.SceneComponent|GetRelativeLocation _sprite))
  ;[1 1 1] Kill Self
  (CallFunction|InputShootRelease)
  (Components|DestroyComponent (Variables|Default|GetCapsuleComponent))
  (Components|DestroyComponent (Variables|Default|GetSight))
  (|CallParentFunction)
  (Transformation|Teleport _armhand (Math|Vector|MakeVector (.x (.location _returnvalue)) -3.0 (.z (.location _returnvalue))) (.rotation _returnvalue))
  (Components|MoveComponentTo _sprite (Math|Vector|MakeVector (.x _relativelocation) -7.0 (.z _relativelocation)) (.rotation (Transformation|GetWorldTransform _sprite)) false false 0.0 true))

(fn ConstructionScript
  (|CallParentFunction))