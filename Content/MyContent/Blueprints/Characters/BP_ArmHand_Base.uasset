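; Base arm-and-hand Blueprint for a BP_Character_Base owner, showing Paper2D flipbooks for holding, reloading, vaulting and dying.
; Every tick it picks a flipbook from vault state, the held gun's holding style (rifle or shotgun) and gun state, with Fire reusing the idle art.
; Reload and Die events use fixed delays to time their animations, and facing events shift the flipbook to either side.
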(event Custom|Update%20Animation
  ;[1 1 1] Handle Animation
  (if (Variables|Default|GetAHIsAlive)
    (bind _asbp_character_base (Utilities|Casting|CastToBP_Character_Base (Components|GetOwner)))
    (if (Variables|Default|GetIsVaulting)
      (Sprite|SetFlipbook (Variables|Default|GetArmHandFlipbook) "/Game/MyContent/Flipbooks/Merc_Vault_ArmHand_Flipbook.Merc_Vault_ArmHand_Flipbook")
      (else
        (switch int (Variables|/Game/MyContent/Blueprints/Weapons/BP_Gun.BP_Gun_C|GetHoldingStyle (Variables|/Game/MyContent/Blueprints/Characters/BP_Character_Base.BP_Character_Base_C|GetHeldGun _asbp_character_base))
          (:0
            (switch Utilities|FlowControl|Switch|SwitchonAH_Gun_States (Variables|Default|GetGunStates)
              (:NewEnumerator0
                (Sprite|SetFlipbook (Variables|Default|GetArmHandFlipbook) (Variables|Default|GetIdle_Rifle_FB)))
              (:NewEnumerator5
                (Sprite|SetFlipbook (Variables|Default|GetArmHandFlipbook) (Variables|Default|GetIdle_Rifle_FB)))
              (:NewEnumerator6
                (Sprite|SetFlipbook (Variables|Default|GetArmHandFlipbook) (Variables|Default|GetReloading_Rifle_FB)))))
          (:1
            (switch Utilities|FlowControl|Switch|SwitchonAH_Gun_States (Variables|Default|GetGunStates)
              (:NewEnumerator0
                (Sprite|SetFlipbook (Variables|Default|GetArmHandFlipbook) (Variables|Default|GetIdle_Shotgun_FB)))
              (:NewEnumerator5
                (Sprite|SetFlipbook (Variables|Default|GetArmHandFlipbook) (Variables|Default|GetIdle_Shotgun_FB)))
              (:NewEnumerator6
                (Sprite|SetFlipbook (Variables|Default|GetArmHandFlipbook) (Variables|Default|GetReloading_Shotgun_FB))))))))))

(event Custom|Reload
  ;[1 1 1] Reload
  (Variables|Default|SetIsReloading true)
  (Variables|Default|SetGunStates "NewEnumerator6")
  (CallFunction|UpdateAnimation)
  (Utilities|FlowControl|Delay 1.4)
  (Variables|Default|SetGunStates "NewEnumerator0")
  (CallFunction|UpdateAnimation))

(event Custom|RightFacing
  ;[1 1 1] Set Facing
  (Components|MoveComponentTo (Variables|Default|GetArmHandFlipbook) "0,1.500000,23.000000" "0, 0, 0" false false 0.0 false))

(event Custom|Die
  ;[1 1 1] Die
  (Variables|Default|SetAHIsAlive false)
  (Sprite|SetFlipbook (Variables|Default|GetArmHandFlipbook) (Variables|Default|GetDying_FB))
  (Utilities|FlowControl|Delay 0.8)
  (Sprite|SetFlipbook (Variables|Default|GetArmHandFlipbook) (Variables|Default|GetDead_FB)))

(event Custom|LeftFacing
  ;[1 1 1] Set Facing
  (Components|MoveComponentTo (Variables|Default|GetArmHandFlipbook) "0,-1.500000,23.000000" "0, 0, 0" false false 0.0 false))

(event EventTick
  (params (DeltaSeconds :type Float%20%28single-precision%29))
  ;[1 1 1] Event Tick
  (CallFunction|UpdateAnimation))

(fn ConstructionScript)