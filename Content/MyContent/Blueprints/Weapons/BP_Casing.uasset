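; BP_Casing is a weapon shell casing, drawn as a Paper2D sprite chosen by CasingType.
; On spawn it reads the owning BP_Character_Base and launches via ProjectileMovement, adding an upward kick and random sideways push opposite the facing to the character's velocity.
; It destroys itself after a short delay, or sooner when its box overlaps an actor with "TileMap" in its display name.
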(event OnComponentBeginOverlap(Box)
  (params (OverlappedComponent :type Primitive%20Component%20Object%20Reference) (OtherActor :type Actor%20Object%20Reference) (OtherComp :type Primitive%20Component%20Object%20Reference) (OtherBodyIndex :type Integer) (bFromSweep :type Boolean) (SweepResult :type Hit%20Result%20Structure%20%28by%20ref%29))
  ;[1 1 1] Destroy on Hit Ground
  (if (Utilities|String|Contains (Utilities|GetDisplayName OtherActor) "TileMap")
    (Actor|DestroyActor)))

(event Custom|Spawn
  ;[1 1 1] Event BeginPlay
  (Rendering|Components|Sprite|SetSprite (Variables|Default|GetPaperSprite) (Variables|Default|GetCasingType))
  (bind _asbp_character_base (Utilities|Casting|CastToBP_Character_Base (Components|GetOwner)))
  (if (Variables|/Game/MyContent/Blueprints/Characters/BP_Character_Base.BP_Character_Base_C|GetIsMovingRight _asbp_character_base)
    (Variables|Default|SetDirection -1.0)
    (else
      (Variables|Default|SetDirection 1.0)))
  (Game|Components|ProjectileMovement|SetVelocityinLocalSpace (Variables|Default|GetProjectileMovement) (Math|Vector|MakeVector (+ (.x (Variables|/Script/Engine.MovementComponent|GetVelocity (Variables|/Script/Engine.Character|GetCharacterMovement _asbp_character_base))) (* (Variables|Default|GetDirection) (Math|Random|RandomFloatinRange 2e+01 5e+01))) 0.0 (+ (.z (Variables|/Script/Engine.MovementComponent|GetVelocity (Variables|/Script/Engine.Character|GetCharacterMovement _asbp_character_base))) 8e+01)))
  (Utilities|FlowControl|Delay 1.2)
  (Actor|DestroyActor))

(fn ConstructionScript)