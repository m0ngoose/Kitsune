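; BP_BloodSpurt is a short-lived Paper2D blood spurt effect owned by a BP_Bullet.
; On BeginPlay it sets its sprite from CasingType, destroys the bullet's root component and launches itself opposite the shooting direction at a randomized local X speed.
; It destroys itself after a short delay, or earlier when its box overlaps an actor whose display name contains "TileMap".
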(event OnComponentBeginOverlap(Box)
  (params (OverlappedComponent :type Primitive%20Component%20Object%20Reference) (OtherActor :type Actor%20Object%20Reference) (OtherComp :type Primitive%20Component%20Object%20Reference) (OtherBodyIndex :type Integer) (bFromSweep :type Boolean) (SweepResult :type Hit%20Result%20Structure%20%28by%20ref%29))
  ;[1 1 1] Destroy on Hit Ground
  (if (Utilities|String|Contains (Utilities|GetDisplayName OtherActor) "TileMap")
    (Actor|DestroyActor)))

(event EventBeginPlay
  ;[1 1 1] Event BeginPlay
  (Rendering|Components|Sprite|SetSprite (Variables|Default|GetPaperSprite) (Variables|Default|GetCasingType))
  (bind _asbp_bullet (Utilities|Casting|CastToBP_Bullet (Components|GetOwner)))
  (if (Variables|/Game/MyContent/Blueprints/Weapons/BP_Bullet.BP_Bullet_C|GetShootingRight _asbp_bullet)
    (Variables|Default|SetDirection -1.0)
    (else
      (Variables|Default|SetDirection 1.0)))
  (Components|DestroyComponent (Variables|/Script/Engine.Actor|GetRootComponent _asbp_bullet) _asbp_bullet)
  (Game|Components|ProjectileMovement|SetVelocityinLocalSpace (Variables|Default|GetProjectileMovement) (Math|Vector|MakeVector (* (Variables|Default|GetDirection) (Math|Random|RandomFloatinRange 4e+01 6e+01)) 0.0 0.0))
  (Utilities|FlowControl|Delay 1.2)
  (Actor|DestroyActor))

(fn ConstructionScript)