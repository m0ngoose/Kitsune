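; Projectile fired by BP_Gun that damages characters in side-on combat along the X axis.
; On BeginPlay it takes shooter, damage and speed from its owning gun, then sets velocity left or right from the sign of its yaw.
; Overlapping another character's Cylinder component, matched by display name, removes health, spawns blood spurts and destroys the bullet.
; An ApplyKnockback call is present but never runs.
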(event OnComponentBeginOverlap(Box)
  (params (OverlappedComponent :type Primitive%20Component%20Object%20Reference) (OtherActor :type Actor%20Object%20Reference) (OtherComp :type Primitive%20Component%20Object%20Reference) (OtherBodyIndex :type Integer) (bFromSweep :type Boolean) (SweepResult :type Hit%20Result%20Structure%20%28by%20ref%29))
  (bind _returnvalue (Transformation|GetActorLocation))
  ;[1 1 1] Hits Player
  (if (!= OtherActor (Variables|Default|GetFiredBy))
    (if (Utilities|String|Contains (Utilities|GetDisplayName OtherComp) "Cylinder")
      (bind _asbp_character_base (Utilities|Casting|CastToBP_Character_Base OtherActor))
      (Default|RemoveHealth _asbp_character_base (Variables|Default|GetBullet%20Damage))
      (for _index (range 0 2)
        (Game|SpawnActorfromClass "/Game/MyContent/Blueprints/Weapons/BP_BloodSpurt.BP_BloodSpurt_C" (Math|Transform|MakeTransform (Math|Vector|MakeVector (.x _returnvalue) (.y _returnvalue) (+ (.z _returnvalue) (Math|Random|RandomFloatinRange -1.0 1.0))) "0, 0, 0" "1,1,1") "AlwaysSpawn" self 0))
      (Actor|DestroyActor))))

(event EventBeginPlay
  (bind _projectilemovement (Variables|Default|GetProjectileMovement))
  ;[1 1 1] Event BeginPlay
  (bind _asbp_gun (Utilities|Casting|CastToBP_Gun (Components|GetOwner)))
  (Variables|Default|SetFiredBy (Variables|/Game/MyContent/Blueprints/Weapons/BP_Gun.BP_Gun_C|GetWeaponHolder _asbp_gun))
  (Variables|Default|SetBullet%20Damage (Variables|/Game/MyContent/Blueprints/Weapons/BP_Gun.BP_Gun_C|GetBulletDamage _asbp_gun))
  (if (< (.yaw (Transformation|GetActorRotation)) 0.0)
    (Variables|/Script/Engine.MovementComponent|SetVelocity _projectilemovement (Math|Vector|MakeVector (* -1.0 (Variables|/Game/MyContent/Blueprints/Weapons/BP_Gun.BP_Gun_C|GetBulletSpeed _asbp_gun)) 0.0 0.0))
    (Variables|Default|SetShootingRight false)
    (else
      (Variables|/Script/Engine.MovementComponent|SetVelocity _projectilemovement (Math|Vector|MakeVector (Variables|/Game/MyContent/Blueprints/Weapons/BP_Gun.BP_Gun_C|GetBulletSpeed _asbp_gun) 0.0 0.0))
      (Variables|Default|SetShootingRight true))))

(fn ConstructionScript)