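; Base-style 2D gun actor that fires bullets, tracks magazine and reserve ammo, and pushes ammo and reload state to its owning BP_Character_Base.
; Fire spawns a bullet and casing, plays first or random shot sounds, optionally applies knockback and auto-reloads when empty.
; Reload runs on timed delays, and a state enum selects the Paper2D flipbook.
; Facing events shift the sprite's depth, and falling stops upon overlapping a TileMap.
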(event OnComponentBeginOverlap(Box)
  (params (OverlappedComponent :type Primitive%20Component%20Object%20Reference) (OtherActor :type Actor%20Object%20Reference) (OtherComp :type Primitive%20Component%20Object%20Reference) (OtherBodyIndex :type Integer) (bFromSweep :type Boolean) (SweepResult :type Hit%20Result%20Structure%20%28by%20ref%29))
  (bind _falldown (Variables|Default|GetFallDown))
  ;[1 1 1] Detect Ground Reached
  (if (Utilities|String|Contains (Utilities|GetDisplayName OtherActor) "TileMap")
    (Game|Components|ProjectileMovement|SetVelocityinLocalSpace _falldown "0, 0, 0")
    (Components|Activation|Deactivate _falldown)))

(event Custom|UpdateAnimation
  ;[1 1 1] Handle Animation
  (switch Utilities|FlowControl|Switch|SwitchonAH_Gun_States (Variables|Default|GetStates)
    (:NewEnumerator0
      (Sprite|SetFlipbook (Variables|Default|GetPaperFlipbook) (Variables|Default|GetIdleFB)))
    (:NewEnumerator5
      (Sprite|SetFlipbook (Variables|Default|GetPaperFlipbook) (Variables|Default|GetFiringFB)))
    (:NewEnumerator6
      (Sprite|SetFlipbook (Variables|Default|GetPaperFlipbook) (Variables|Default|GetReloadingFB)))))

(event Custom|Fire
  (bind _returnvalue (Transformation|GetActorLocation))
  ;[1 1 1] Fire
  (if (not (Variables|Default|GetIsReloading))
    (if (<= (Variables|Default|GetCurrentAmmo) 0)
      (Audio|PlaySoundatLocation (Variables|Default|GetDryShotSd) (Transformation|GetActorLocation) "0, 0, 0" 1.0 1.0 0.0 0 0 0)
      (else
        (Game|SpawnActorfromClass (Variables|Default|GetBulletType) (Transformation|GetWorldTransform (Variables|Default|GetBulletSpawn)) "Undefined" self 0)
        (Variables|Default|SetStates "NewEnumerator5")
        (CallFunction|RemoveAmmo)
        (CallFunction|UpdateAnimation)
        (bind _asbp_character_base (Utilities|Casting|CastToBP_Character_Base (Components|GetOwner)))
        (if (Variables|/Game/MyContent/Blueprints/Characters/BP_Character_Base.BP_Character_Base_C|GetIsFirstShot _asbp_character_base)
          (Audio|PlaySoundatLocation (Variables|Default|GetFirstShotSd) _returnvalue "0, 0, 0" 1.0 1.0 0.0 0 0 0)
          (else
            (Audio|PlaySoundatLocation (Variables|Default|GetRdmShotSd) _returnvalue "0, 0, 0" 1.0 1.0 0.0 0 0 0)))
        (if (Variables|Default|GetKnockback)
          (bind _asbp_character_base_2 (Utilities|Casting|CastToBP_Character_Base (Components|GetOwner)))
          (Default|ApplyKnockback _asbp_character_base_2 0.0))
        (bind _returnvalue_2 (Game|SpawnActorfromClass "/Game/MyContent/Blueprints/Weapons/BP_Casing.BP_Casing_C" (Math|Transform|MakeTransform (+ (Transformation|GetActorLocation) "0.000000,3.000000, 0") (* (Transformation|GetActorRotation _asbp_character_base_2) 1)) "AlwaysSpawn" (Components|GetOwner) 0))
        (Variables|/Game/MyContent/Blueprints/Weapons/BP_Casing.BP_Casing_C|SetCasingType _returnvalue_2 (Variables|Default|GetCasingType))
        (Default|Spawn _returnvalue_2)
        (Utilities|FlowControl|Delay 0.25)
        (Variables|Default|SetStates "NewEnumerator0")
        (CallFunction|UpdateAnimation)
        (CallFunction|UpdateOwningCharacter)
        (if (Variables|Default|GetAutoReload)
          (if (<= (Variables|Default|GetCurrentAmmo) 0)
            (if (> (Variables|Default|GetReserveAmmo) 0)
              (CallFunction|Reload)
              (Utilities|Casting|CastToBP_Character_Base (Components|GetOwner)))))))))

(event Custom|RightFacing
  (bind _paperflipbook (Variables|Default|GetPaperFlipbook))
  (bind _relativelocation (Variables|/Script/Engine.SceneComponent|GetRelativeLocation _paperflipbook))
  ;[1 1 1] Set Facing
  (Components|MoveComponentTo _paperflipbook (Math|Vector|MakeVector (.x _relativelocation) 0.5 (.z _relativelocation)) "0, 0, 0" false false 0.0 false)
  (Variables|Default|SetFacingRight true))

(event Custom|Reload
  ;[1 1 1] Reload
  (Variables|Default|SetIsReloading true)
  (CallFunction|UpdateOwningCharacter)
  (Audio|PlaySoundatLocation (Variables|Default|GetUnloadSd) (Transformation|GetActorLocation) "0, 0, 0" 1.0 1.0 0.0 0 0 0)
  (Variables|Default|SetStates "NewEnumerator6")
  (CallFunction|UpdateAnimation)
  (Utilities|FlowControl|Delay 1.1)
  (Audio|PlaySoundatLocation (Variables|Default|GetLoadSd) (Transformation|GetActorLocation) "0, 0, 0" 1.0 1.0 0.0 0 0 0)
  (Utilities|FlowControl|Delay 0.3)
  (Variables|Default|SetStates "NewEnumerator0")
  (CallFunction|UpdateAnimation)
  (Variables|Default|SetLostAmmo (- (Variables|Default|GetMaxAmmo) (Variables|Default|GetCurrentAmmo)))
  (if (>= (Variables|Default|GetReserveAmmo) (Variables|Default|GetLostAmmo))
    (Variables|Default|SetReserveAmmo (- (Variables|Default|GetReserveAmmo) (Variables|Default|GetLostAmmo)))
    (Variables|Default|SetCurrentAmmo (Variables|Default|GetMaxAmmo))
    (else
      (Variables|Default|SetCurrentAmmo (+ (Variables|Default|GetCurrentAmmo) (Variables|Default|GetReserveAmmo)))
      (Variables|Default|SetReserveAmmo 0)))
  (Variables|Default|SetIsReloading false)
  (CallFunction|UpdateOwningCharacter))

(event Custom|Update%20Owning%20Character
  ;[1 1 1] Update Owning Character
  (bind _asbp_character_base (Utilities|Casting|CastToBP_Character_Base (Components|GetOwner)))
  (Variables|/Game/MyContent/Blueprints/Characters/BP_Character_Base.BP_Character_Base_C|SetAmmoCount _asbp_character_base (Variables|Default|GetCurrentAmmo))
  (Variables|/Game/MyContent/Blueprints/Characters/BP_Character_Base.BP_Character_Base_C|SetAmmoReserve _asbp_character_base (Variables|Default|GetReserveAmmo))
  (Variables|/Game/MyContent/Blueprints/Characters/BP_Character_Base.BP_Character_Base_C|SetIsReloading _asbp_character_base (Variables|Default|GetIsReloading)))

(event Custom|Restock%20Ammo
  ;[1 1 1] Restock Ammo
  (Variables|Default|SetReserveAmmo (Variables|Default|GetInitialReserve))
  (CallFunction|UpdateOwningCharacter))

(event Custom|LeftFacing
  (bind _paperflipbook (Variables|Default|GetPaperFlipbook))
  (bind _relativelocation (Variables|/Script/Engine.SceneComponent|GetRelativeLocation _paperflipbook))
  ;[1 1 1] Set Facing
  (Components|MoveComponentTo _paperflipbook (Math|Vector|MakeVector (.x _relativelocation) -0.5 (.z _relativelocation)) "0, 0, 0" false false 0.0 false)
  (Variables|Default|SetFacingRight false))

(event Custom|Enable%20Gravity
  ;[1 1 1] Enable Gravity
  (Components|Activation|Activate (Variables|Default|GetFallDown) false))

(event EventTick
  (params (DeltaSeconds :type Float%20%28single-precision%29))
  ;[1 1 1] Event Tick
  (CallFunction|UpdateAnimation))

(event EventBeginPlay
  ;[1 1 1] Event Begin Play
  (Variables|Default|SetCurrentAmmo (Variables|Default|GetMaxAmmo))
  (Variables|Default|SetReserveAmmo (Variables|Default|GetInitialReserve))
  (Variables|Default|SetWeaponHolder (Components|GetOwner self)))

(fn ConstructionScript)

(fn RemoveAmmo
  (Variables|Default|SetCurrentAmmo (- (Variables|Default|GetCurrentAmmo) 1)))